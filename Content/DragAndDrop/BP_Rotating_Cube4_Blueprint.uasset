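; Cube actor Blueprint that moves itself repeatedly between two locations; despite its name, the graph applies no rotation.
; BeginPlay checks the Start and End components and caches their world locations once, so the targets stay fixed as the actor moves.
; The LerpPosition timeline drives a non-swept vector lerp between those points and replays from its start whenever it finishes, looping indefinitely.
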(event Custom|PlayLerp
  (bind _lerping (Timeline|LerpPosition PlayFromStart)
    (:Update
      (Variables|Default|Setlerp _lerping)
      (Transformation|SetActorLocation (Math|Vector|Lerp(Vector) (Variables|Default|GetStart%20point) (Variables|Default|GetEnd%20Point) (Variables|Default|Getlerp)) false false))
    (:Finished
      (CallFunction|PlayLerp))))

(event EventBeginPlay
  (|CallParentFunction)
  (bind _start (Variables|Default|GetStart)
    (:then
      (Variables|Default|SetStart%20point (Transformation|GetWorldLocation _start))
      (bind _end (Variables|Default|GetEnd)
        (:then
          (Variables|Default|SetEnd%20Point (Transformation|GetWorldLocation _end))
          (CallFunction|PlayLerp))
        (:else)))
    (:else)))

(event Collision|EventActorBeginOverlap
  (params (OtherActor :type Actor%20Object%20Reference))
  (|CallParentFunction OtherActor) ; This node is disabled and will not be called.\nDrag off pins to build functionality.
)

(event EventTick
  (params (DeltaSeconds :type Float%20%28single-precision%29))
  (|CallParentFunction DeltaSeconds) ; This node is disabled and will not be called.\nDrag off pins to build functionality.
)

(fn ConstructionScript
  (|CallParentFunction))